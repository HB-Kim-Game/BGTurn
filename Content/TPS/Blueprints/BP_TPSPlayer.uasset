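; Blueprint for the TPS player that registers its Enhanced Input mapping context when play begins.
; BeginPlay casts the controller to a PlayerController and adds IMC_Default to that player's Enhanced Input subsystem.
; Look and movement nodes, including a control-rotation-relative direction calculation, are left unconnected and never run.
; Tick and the construction script are empty.
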(event EventBeginPlay
  (bind _asplayer_controller (Utilities|Casting|CastToPlayerController (Pawn|GetController)))
  (Input|AddMappingContext (PlayerController|LocalPlayerSubsystems|GetEnhancedInputLocalPlayerSubsystem _asplayer_controller) "/Game/ThirdPerson/Input/IMC_Default.IMC_Default" 0 "(bIgnoreAllPressedKeysUntilRelease=True,bForceImmediately=False,bNotifyUserSettings=False)"))

(event Collision|EventActorBeginOverlap
  (params (OtherActor :type Actor%20Object%20Reference)))

(event EventTick
  (params (DeltaSeconds :type Float%20%28single-precision%29)))

(fn ConstructionScript)